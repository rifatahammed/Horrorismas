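; Level 1 game state Blueprint that tracks an ordered list of objectives and drives the objective display on the main HUD.
; The current objective is the first uncompleted entry in the array, and Initialize stores the HUD reference and shows it.
; Completion and next-objective events act only when the passed ID matches the current objective.
; Completing flags the entry and hides the widget, optionally showing the next objective immediately or leaving that to a later call.
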(event EventBeginPlay)

(event EventTick
  (params (DeltaSeconds :type Float%20%28single-precision%29)))

(event EventCompleteObjectiveCall
  (params (ObjectiveID :type Name :default "None") (SetNextObjectiveImmediately :type Boolean))
  (if (== ObjectiveID (.idname (CallFunction|FindCurrentObjective)))
    (CallFunction|CompleteObjective)
    (if SetNextObjectiveImmediately
      (CallFunction|SetObjective))))

(event EventSetNextObjective
  (params (ObjectiveID :type Name :default "None"))
  (if (== ObjectiveID (.idname (CallFunction|FindCurrentObjective)))
    (CallFunction|SetObjective)))

(fn ConstructionScript)

(fn FindCurrentObjective
  (bind _array_element (Utilities|Array|ForEachLoopwithBreak (Variables|Default|GetObjectives) :!label _label)
    (:LoopBody
      (if (not (.ObjectiveCompleted (Utilities|Struct|BreakS_ObjectiveData _array_element)))
        (LocalVariables|SetLocalObjective _array_element)
        (goto _label Break)))
    (:Completed
      (return (LocalVariables|GetLocalObjective)))))

(fn Initialize
  (params (MainHud :type W%20Main%20Hud%20Object%20Reference))
  (Variables|Default|SetMain%20HudRef MainHud)
  (CallFunction|SetObjective)
  (return))

(fn SetObjective
  (bind _main_hudref (Variables|Default|GetMain%20HudRef))
  (bind _w_objectives (Variables|/Game/_Game/UMG/W_MainHud.W_MainHud_C|GetW_Objectives _main_hudref))
  (Default|UpdateObjectiveText _w_objectives (.objectivetitle (CallFunction|FindCurrentObjective)))
  (Widget|SetVisibility _w_objectives "SelfHitTestInvisible")
  (return))

(fn CompleteObjective
  (bind _localobjective1 (CallFunction|FindCurrentObjective))
  (bind _objectives (Variables|Default|GetObjectives))
  (bind (_idname _objectivetitle) (Utilities|Struct|BreakS_ObjectiveData _localobjective1))
  (Utilities|Array|SetArrayElem _objectives (Utilities|Array|FindItem _objectives _localobjective1) (Utilities|Struct|MakeS_ObjectiveData _idname _objectivetitle true))
  (Widget|SetVisibility (Variables|/Game/_Game/UMG/W_MainHud.W_MainHud_C|GetW_Objectives (Variables|Default|GetMain%20HudRef)) "Hidden")
  (return))