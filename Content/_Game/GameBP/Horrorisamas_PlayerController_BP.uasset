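; Player controller for Horrorisamas that handles mouse look and the inventory menu.
; On BeginPlay it creates the inventory widget hidden, and look axes scale by a sensitivity value.
; The inventory toggle, gated by a can-open flag, freezes movement and look, shows the cursor, removes any examination widget and switches to game-and-UI input, then reverses on close.
; The Return key broadcasts a PressedReturn event for other listeners.
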(event Custom|ToggleInventory
  (bind _returnvalue (Game|GetPlayerCharacter 0))
  (bind _self self)
  (bind _inventorymenuwidgetref (Variables|Default|GetInventoryMenuWidgetRef))
  (bind _examinationwidgetref (Variables|Default|GetExaminationWidgetRef))
  (bind _charactermovement (Variables|/Script/Engine.Character|GetCharacterMovement _returnvalue))
  (if (Variables|Default|GetCanOpenInventory)
    (if (Variables|Default|GetisInventoryOpen)
      (Variables|Default|SetisInventoryOpen false)
      (Pawn|Components|CharacterMovement|SetMovementMode _charactermovement "MOVE_Walking" 0)
      (Input|ResetIgnoreLookInput)
      (Variables|Default|SetbShowMouseCursor false)
      (Widget|SetVisibility _inventorymenuwidgetref "Collapsed")
      (Input|SetInputModeGameOnly _self)
      (else
        (Variables|Default|SetisInventoryOpen true)
        (Pawn|Components|CharacterMovement|DisableMovement _charactermovement)
        (Input|SetIgnoreLookInput true)
        (Variables|Default|SetbShowMouseCursor true)
        (Widget|SetVisibility _inventorymenuwidgetref "SelfHitTestInvisible")
        (if (UserInterface|Viewport|IsinViewport _examinationwidgetref)
          (Widget|RemovefromParent _examinationwidgetref))
        (Input|SetInputModeGameandUI _self (Variables|Default|GetInventoryMenuWidgetRef) "DoNotLock" true)))))

(event EventBeginPlay
  (bind _returnvalue (UserInterface|CreateWidget "/Game/_Game/UMG/Inventory/InventoryMenuWidget.InventoryMenuWidget_C"))
  (bind _output_get (Variables|Default|SetInventoryMenuWidgetRef _returnvalue))
  (Widget|SetVisibility _output_get "Collapsed")
  (UserInterface|Viewport|AddtoViewport (Variables|Default|GetInventoryMenuWidgetRef) 0))

(event Input|ActionEvents|InputActionInventoryToggle
  (params (Key :type Key%20Structure :default "None"))
  (:Pressed
    (CallFunction|ToggleInventory)))

(event Input|ActionEvents|InputActionReturn
  (params (Key :type Key%20Structure :default "None"))
  (:Pressed
    (Default|CallPressedReturn)))

(event Input|AxisEvents|InputAxisLookUp
  (params (AxisValue :type Float%20%28single-precision%29))
  (Class|PlayerController|AddPitchInput (* AxisValue (Variables|Default|GetLookSensitivity))))

(event Input|AxisEvents|InputAxisLookRight
  (params (AxisValue :type Float%20%28single-precision%29))
  (Class|PlayerController|AddYawInput (* AxisValue (Variables|Default|GetLookSensitivity))))

(fn ConstructionScript)