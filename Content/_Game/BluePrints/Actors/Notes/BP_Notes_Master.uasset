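; BP_Notes_Master is a note actor, apparently a base for readable notes, that shows an interaction prompt and opens an examination UI.
; OverlapSphere enables per-tick visibility traces to the player camera, showing a camera-facing prompt when unobstructed and enabling input within PickUpDistance.
; The Action input creates a NoteExaminationWidget, passing it this note and the level's BP_NoteExamination actor.
; The construction script applies the note's text.
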(event OnComponentBeginOverlap(OverlapSphere)
  (params (OverlappedComponent :type Primitive%20Component%20Object%20Reference) (OtherActor :type Actor%20Object%20Reference) (OtherComp :type Primitive%20Component%20Object%20Reference) (OtherBodyIndex :type Integer) (bFromSweep :type Boolean) (SweepResult :type Hit%20Result%20Structure%20%28by%20ref%29))
  (bind _asl1_character_bp (Utilities|Casting|CastToL1_Character_BP OtherActor))
  (Variables|Default|SetPlayerRef _asl1_character_bp)
  (Rendering|SetVisibility (Variables|Default|GetPromptWidget) true false)
  (Variables|Default|SetUpdateActor true))

(event OnComponentEndOverlap(OverlapSphere)
  (params (OverlappedComponent :type Primitive%20Component%20Object%20Reference) (OtherActor :type Actor%20Object%20Reference) (OtherComp :type Primitive%20Component%20Object%20Reference) (OtherBodyIndex :type Integer))
  (Utilities|Casting|CastToL1_Character_BP OtherActor)
  (Rendering|SetVisibility (Variables|Default|GetPromptWidget) false false)
  (Variables|Default|SetUpdateActor false)
  (Input|DisableInput (Game|GetPlayerController 0)))

(event EventBeginPlay
  (bind _outactors (Actor|GetAllActorsOfClass "/Game/_Game/BluePrints/Actors/Notes/BP_NoteExamination.BP_NoteExamination_C"))
  (Variables|Default|SetBPNoteExaminationRef (Utilities|Array|Get(acopy) _outactors)))

(event EventTick
  (params (DeltaSeconds :type Float%20%28single-precision%29))
  (bind _returnvalue (Game|GetPlayerController 0))
  (bind _paper (Variables|Default|GetPaper))
  (bind _returnvalue_2 (Transformation|GetWorldLocation _paper))
  (Transformation|SetWorldLocation (Variables|Default|GetPromptWidget) (Math|Vector|MakeVector (.x _returnvalue_2) (.y _returnvalue_2) (+ (.z _returnvalue_2) (Variables|Default|GetWidgetDistanceAboveMesh))) false false)
  (if (Variables|Default|GetUpdateActor)
    (bind (_outhit _returnvalue_3) (Collision|LineTraceByChannel (Transformation|GetActorLocation) (Transformation|GetWorldLocation (Variables|/Game/_Game/GameBP/Level1/L1_Character_BP.L1_Character_BP_C|GetCamera (Variables|Default|GetPlayerRef))) "TraceTypeQuery1" false 0 "None"))
    (if (not _returnvalue_3)
      (Rendering|SetVisibility (Variables|Default|GetPromptWidget) true false)
      (Transformation|SetWorldRotation (Variables|Default|GetPromptWidget) (Math|Rotator|FindLookatRotation (Transformation|GetWorldLocation (Variables|Default|GetPromptWidget)) (Transformation|GetWorldLocation (Variables|/Game/_Game/GameBP/Level1/L1_Character_BP.L1_Character_BP_C|GetCamera (Variables|Default|GetPlayerRef)))) false false)
      (Default|TogglePrompt (.AsPick%20Up%20Promt%20Widget (Utilities|Casting|CastToPickUpPromtWidget (UserInterface|GetUserWidgetObject (Variables|Default|GetPromptWidget)))) (<= (Math|Vector|VectorLength (- (.TraceStart (Collision|BreakHitResult _outhit)) (.TraceEnd (Collision|BreakHitResult _outhit)))) (Variables|Default|GetPickUpDistance)))
      (if (<= (Math|Vector|VectorLength (- (.TraceStart (Collision|BreakHitResult _outhit)) (.TraceEnd (Collision|BreakHitResult _outhit)))) (Variables|Default|GetPickUpDistance))
        (Input|EnableInput _returnvalue)
        (else
          (Input|DisableInput _returnvalue)))
      (else
        (Rendering|SetVisibility (Variables|Default|GetPromptWidget) false false)
        (Input|DisableInput (Game|GetPlayerController 0))))))

(event Input|ActionEvents|InputActionAction
  (params (Key :type Key%20Structure :default "None"))
  (:Pressed
    (bind _returnvalue (UserInterface|CreateWidget "/Game/_Game/UMG/NoteExaminationWidget.NoteExaminationWidget_C" 0 (Variables|Default|GetBPNoteExaminationRef)))
    (Default|UpdateWidget _returnvalue self)
    (UserInterface|Viewport|AddtoViewport _returnvalue 0)))

(fn ConstructionScript
  (Rendering|Components|TextRender|SetText (Variables|Default|GetNoteText) (Variables|Default|GetNoteText%28Text%29)))