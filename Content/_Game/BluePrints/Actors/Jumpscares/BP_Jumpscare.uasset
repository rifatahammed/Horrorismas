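; BP_Jumpscare is a trigger actor that stages a mannequin jumpscare.
; Overlapping its box plays a collapse sound and enables per-tick movement of the mannequin toward an end point at constant speed via VInterpToConstant.
; One second later it sets the game state's next objective message to investigate the noise, then destroys itself.
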(event OnComponentBeginOverlap(Box)
  (params (OverlappedComponent :type Primitive%20Component%20Object%20Reference) (OtherActor :type Actor%20Object%20Reference) (OtherComp :type Primitive%20Component%20Object%20Reference) (OtherBodyIndex :type Integer) (bFromSweep :type Boolean) (SweepResult :type Hit%20Result%20Structure%20%28by%20ref%29))
  (Audio|PlaySound2D "/Game/StarterContent/Audio/Collapse01.Collapse01" 1.0 1.0 0.0 0 0)
  (Variables|Default|SetEnableJumpscare true)
  (Utilities|FlowControl|Delay 1.0)
  (Class|BPIObjectiveCall|SetNextObjective(Message) (Game|GetGameState) "InvestigateNoise")
  (Actor|DestroyActor))

(event EventTick
  (params (DeltaSeconds :type Float%20%28single-precision%29))
  (if (Variables|Default|GetEnableJumpscare)
    (Transformation|SetWorldLocation (Variables|Default|GetMannequin) (Math|Interpolation|VInterptoConstant (Transformation|GetWorldLocation (Variables|Default|GetMannequin)) (Transformation|GetWorldLocation (Variables|Default|GetEndPoint)) DeltaSeconds (Variables|Default|GetSpeed)) false false)))

(fn ConstructionScript)