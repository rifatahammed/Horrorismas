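; BP_HideActor is an interactable hiding spot that moves the player into and out of hiding.
; Interact starts a looping timer at frame-delta interval that interpolates the player toward the HidingPosition or ExitPosition component, chosen by the player's IsHiding flag.
; Collision and movement are disabled before entering.
; On arrival the timers clear and IsHiding flips, with collision and walking restored on exit.
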(event Custom|MoveCharacter
  (bind _playerref (Variables|Default|GetPlayerRef))
  (Transformation|SetActorTransform _playerref (Math|Transform|MakeTransform (Math|Interpolation|VInterpTo (Transformation|GetActorLocation _playerref) (Transformation|GetWorldLocation (select (Variables|/Game/_Game/GameBP/Level1/L1_Character_BP.L1_Character_BP_C|GetisHiding (Variables|Default|GetPlayerRef)) (Variables|Default|GetExitPosition) (Variables|Default|GetHidingPosition))) (Utilities|Time|GetWorldDeltaSeconds) 1e+01) "0, 0, 0" "1.000000,1.000000,1.000000"))
  (if (Utilities|Operators|EqualEqual (Transformation|GetActorLocation (Variables|Default|GetPlayerRef)) (Transformation|GetWorldLocation (select (Variables|/Game/_Game/GameBP/Level1/L1_Character_BP.L1_Character_BP_C|GetisHiding (Variables|Default|GetPlayerRef)) (Variables|Default|GetExitPosition) (Variables|Default|GetHidingPosition))) 0.01)
    (Utilities|Time|ClearandInvalidateTimerbyHandle (stale EventInteract _returnvalue_2))
    (Utilities|Time|ClearandInvalidateTimerbyHandle (stale EventInteract _returnvalue))
    (CallFunction|FinishedMoving)))

(event Custom|FinishedMoving
  (bind _playerref (Variables|Default|GetPlayerRef))
  (bind _playerref_2 (Variables|Default|GetPlayerRef))
  (if (Variables|/Game/_Game/GameBP/Level1/L1_Character_BP.L1_Character_BP_C|GetisHiding _playerref)
    (Variables|/Game/_Game/GameBP/Level1/L1_Character_BP.L1_Character_BP_C|SetisHiding _playerref false)
    (Collision|SetActorEnableCollision _playerref_2 true)
    (Pawn|Components|CharacterMovement|SetMovementMode (Variables|/Script/Engine.Character|GetCharacterMovement _playerref_2) "MOVE_Walking" 0)
    (else
      (Variables|/Game/_Game/GameBP/Level1/L1_Character_BP.L1_Character_BP_C|SetisHiding _playerref true))))

(event EventBeginPlay
  (bind _asl1_character_bp (Utilities|Casting|CastToL1_Character_BP (Game|GetPlayerCharacter 0)))
  (Variables|Default|SetPlayerRef _asl1_character_bp))

(event EventInteract
  (bind _playerref (Variables|Default|GetPlayerRef))
  (if (Variables|/Game/_Game/GameBP/Level1/L1_Character_BP.L1_Character_BP_C|GetisHiding (Variables|Default|GetPlayerRef))
    (bind _returnvalue (Utilities|Time|SetTimerbyEvent (delegate Custom|MoveCharacter) (Utilities|Time|GetWorldDeltaSeconds) true))
    (else
      (Collision|SetActorEnableCollision _playerref false)
      (Pawn|Components|CharacterMovement|DisableMovement (Variables|/Script/Engine.Character|GetCharacterMovement _playerref))
      (bind _returnvalue_2 (Utilities|Time|SetTimerbyEvent (delegate Custom|MoveCharacter) (Utilities|Time|GetWorldDeltaSeconds) true)))))

(fn ConstructionScript)