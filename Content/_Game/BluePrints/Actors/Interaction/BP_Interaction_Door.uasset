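; An interactable door actor that swings open and closed when interacted with.
; The Interact event toggles a closed flag and plays or reverses a timeline.
; The timeline's alpha lerps the static mesh's relative yaw between zero and a quarter turn.
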(event EventBeginPlay
  (|CallParentFunction) ; This node is disabled and will not be called.\nDrag off pins to build functionality.
)

(event Collision|EventActorBeginOverlap
  (params (OtherActor :type Actor%20Object%20Reference))
  (|CallParentFunction OtherActor) ; This node is disabled and will not be called.\nDrag off pins to build functionality.
)

(event EventTick
  (params (DeltaSeconds :type Float%20%28single-precision%29))
  (|CallParentFunction DeltaSeconds) ; This node is disabled and will not be called.\nDrag off pins to build functionality.
)

(event EventInteract
  (if (Variables|Default|GetisDoorClosed)
    (Variables|Default|SetisDoorClosed false)
    (bind _alpha (Timeline|OpenDoorTL Play)
      (:Update
        (Transformation|SetRelativeRotation (Variables|Default|GetStaticMesh) (Math|Rotator|MakeRotator 0.0 0.0 (Math|Float|Lerp 0.0 -9e+01 _alpha)) false false)))
    (else
      (Variables|Default|SetisDoorClosed true)
      (Timeline|OpenDoorTL Reverse))))

(fn ConstructionScript
  (|CallParentFunction))