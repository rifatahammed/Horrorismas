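; BP_PhysicsDoor is a grabbable door that the player swings open with horizontal look input.
; GrabObject disables character movement and look input, then enables input on the door so the LookRight axis feeds MoveDoor.
; MoveDoor adds the axis value directly to the door's relative yaw, with no clamping or physics forces in the graph.
; ReleaseObject restores walking and look input, then disables the door's input.
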(event Custom|MoveDoor
  (params (Amount :type Float%20%28double-precision%29))
  (bind _door (Variables|Default|GetDoor))
  ;[1 1 1] Door Open Rotation
  (Transformation|SetRelativeRotation _door (Math|Rotator|CombineRotators (Variables|/Script/Engine.SceneComponent|GetRelativeRotation _door) (Math|Rotator|MakeRotator 0.0 0.0 Amount)) false false))

(event EventBeginPlay)

(event Collision|EventActorBeginOverlap
  (params (OtherActor :type Actor%20Object%20Reference)))

(event EventTick
  (params (DeltaSeconds :type Float%20%28single-precision%29)))

(event EventGrabObject
  (bind _returnvalue (Game|GetPlayerController 0))
  ;[1 1 1] Disable Camera and Movement When Left click on door
  (Pawn|Components|CharacterMovement|DisableMovement (Variables|/Script/Engine.Character|GetCharacterMovement (Game|GetPlayerCharacter 0)))
  (Input|SetIgnoreLookInput _returnvalue true)
  (Input|EnableInput _returnvalue))

(event EventReleaseObject
  (bind _returnvalue (Game|GetPlayerController 0))
  ;[1 1 1] Re Enabling Character Movement
  (Pawn|Components|CharacterMovement|SetMovementMode (Variables|/Script/Engine.Character|GetCharacterMovement (Game|GetPlayerCharacter 0)) "MOVE_Walking" 0)
  (Input|ResetIgnoreLookInput _returnvalue)
  (Input|DisableInput _returnvalue))

(event Input|AxisEvents|InputAxisLookRight
  (params (AxisValue :type Float%20%28single-precision%29))
  ;[1 1 1] Mouse Move to Open Door
  (CallFunction|MoveDoor AxisValue))

(fn ConstructionScript)